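; Actor component that fetches live local weather from the AMap (Gaode) REST API through the VaRest plugin.
; InitWeatherByURL first looks up the caller's adcode and city by IP, then chains a second GET request using that adcode.
; The final callback reads the "lives" array and stores weather, temperature, wind direction and wind power in component variables.
; GetVaRest wraps a validity check around the VaRest subsystem used for both calls.
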(event `InitWeatherByURL`
  (`self.GetCityInfoByIP`))

(event `GetCityInfoByIP`
  (bind _returnvalue (`self.GetVaRest`)
    (:`Is Valid`
      (`VaRestSubsystem.CallURL` _returnvalue (`KismetTextLibrary.Conv_TextToString` (`|FormatText` "https://restapi.amap.com/v3/ip?&key={Key}" (`self.Key`))) "GET" "x_www_form_urlencoded_url" null (delegate `OnGetAdCodeAndCity`)))))

(event `OnGetAdCodeAndCity`
  (params (Request :type "VaRestRequestJSON Object Reference"))
  (bind _returnvalue (`VaRestRequestJSON.GetResponseObject` Request))
  (bind _output_get (set `self.AdCode` (`VaRestJsonObject.GetStringField` _returnvalue "adcode")))
  (set `self.City` (`VaRestJsonObject.GetStringField` _returnvalue "city"))
  (`self.GetWeatherInfoByAdCode` _output_get))

(event `GetWeatherInfoByAdCode`
  (params (AdCode :type String))
  (bind _returnvalue (`self.GetVaRest`)
    (:`Is Valid`
      (`VaRestSubsystem.CallURL` _returnvalue (`KismetTextLibrary.Conv_TextToString` (`|FormatText` "https://restapi.amap.com/v3/weather/weatherInfo?city={AdCode}&key={Key}" AdCode (`self.Key`))) "GET" "x_www_form_urlencoded_url" null (delegate `OnGetWeatherInfo`)))))

(event `OnGetWeatherInfo`
  (params (Request :type "VaRestRequestJSON Object Reference"))
  (for _array_element (`VaRestJsonObject.GetObjectArrayField` (`VaRestRequestJSON.GetResponseObject` Request) "lives")
    (set `self.weather` (`VaRestJsonObject.GetStringField` _array_element "weather"))
    (set `self.temperature` (`VaRestJsonObject.GetStringField` _array_element "temperature"))
    (set `self.winddirection` (`VaRestJsonObject.GetStringField` _array_element "winddirection"))
    (set `self.windpower` (`VaRestJsonObject.GetStringField` _array_element "windpower"))))