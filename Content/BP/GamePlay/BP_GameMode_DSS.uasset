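; Game mode that controls the Ultra Dynamic Sky and Weather environment and the player's input mode.
; On BeginPlay it starts a weather and city fetch by URL through a VaRest component, sets game-only input, and caches the sky, weather and player controller.
; A looping timer advances time of day by TimeSpeed when updates are enabled, wrapping at day's end.
; Preset events trigger timed weather transitions, and a getter exposes the component's weather data.
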(event `ChangeInputMode`
  (params (IsGameMode :type Boolean))
  ;[1 1 1] Change User Input Mode
  (`self.ChangInput` IsGameMode))

(event `self.ReceiveBeginPlay`
  ;[1 1 1] Init
  (`|ExecutionSequence`
    (:`then_0`
      (`self.UpdateWeatherAndCityInfo`)
      (`self.ChangeInputMode` true))
    (:`then_1`
      (bind _returnvalue (`GameplayStatics.GetActorOfClass` "/Game/UltraDynamicSky/Blueprints/Ultra_Dynamic_Weather.Ultra_Dynamic_Weather_C"))
      (`/Engine/EditorBlueprintResources/StandardMacros.IsValid` _returnvalue
        (:`Is Valid`
          (set `self.UD_Weather` _returnvalue)
          (set `self.TimeSpeed` 0.0)
          (set `self.IsTimeCanUpdate` false))))
    (:`then_2`
      (bind _returnvalue_2 (`GameplayStatics.GetActorOfClass` "/Game/UltraDynamicSky/Blueprints/Ultra_Dynamic_Sky.Ultra_Dynamic_Sky_C"))
      (`/Engine/EditorBlueprintResources/StandardMacros.IsValid` _returnvalue_2
        (:`Is Valid`
          (bind _output_get (set `self.UD_Sky` _returnvalue_2))
          (set `/Game/UltraDynamicSky/Blueprints/Ultra_Dynamic_Sky.Time of Day` 1200.0 _output_get)
          (set `/Game/UltraDynamicSky/Blueprints/Ultra_Dynamic_Sky.Animate Time of Day` false _output_get)
          (`KismetSystemLibrary.K2_SetTimerDelegate` (delegate `UpdateSkyTime`) (`self.UpdateFeq`) true))))
    (:`then_3`
      (bind _asbp_player_controller_dss (cast `/Game/BP/GamePlay/BP_PlayerController_DSS` (`GameplayStatics.GetPlayerController` 0)))
      (`/Engine/EditorBlueprintResources/StandardMacros.IsValid` _asbp_player_controller_dss
        (:`Is Valid`
          (set `self.PC_DSS` _asbp_player_controller_dss))))))

(event `UpdateWeatherAndCityInfo`
  (bind _bp_component_varest (`self.BP_Component_VaRest`))
  ;[1 1 1] Update Weather And City Info
  (`/Engine/EditorBlueprintResources/StandardMacros.IsValid` _bp_component_varest
    (:`Is Valid`
      (`/Game/BP/Component/BP_Component_VaRest.InitWeatherByURL` _bp_component_varest))))

(event `UpdateRealTimeSky`
  (params (TimeOfDay :type "Float (double-precision)") (IsActiveAnimateOfDay :type Boolean))
  (bind _ud_sky (`self.UD_Sky`))
  ;[1 1 1] Update Real Time Sky
  (`/Engine/EditorBlueprintResources/StandardMacros.IsValid` _ud_sky
    (:`Is Valid`
      (set `/Game/UltraDynamicSky/Blueprints/Ultra_Dynamic_Sky.Time of Day` TimeOfDay _ud_sky)
      (set `/Game/UltraDynamicSky/Blueprints/Ultra_Dynamic_Sky.Animate Time of Day` IsActiveAnimateOfDay _ud_sky))))

(event `UpdateSkyTime`
  ;[1 1 1] ChangSky
  (if (`self.IsTimeCanUpdate`)
    (`self.ChangeSkyTime`)))

(event `CloseSkyTime`
  (bind _ud_sky (`self.UD_Sky`))
  ;[1 1 1] ChangSky
  (`/Engine/EditorBlueprintResources/StandardMacros.IsValid` _ud_sky
    (:`Is Valid`
      (set `/Game/UltraDynamicSky/Blueprints/Ultra_Dynamic_Sky.Animate Time of Day` false _ud_sky))))

(event `ChangeWeather_Skies`
  ;[1 1 1] ChangeWeather
  (`self.ChangeWeather` "/Game/UltraDynamicSky/Blueprints/Weather_Effects/Weather_Presets/Clear_Skies.Clear_Skies" 5.0))

(event `ChangeWeather_PartlyCloudy`
  ;[1 1 1] ChangeWeather
  (`self.ChangeWeather` "/Game/UltraDynamicSky/Blueprints/Weather_Effects/Weather_Presets/Partly_Cloudy.Partly_Cloudy" 5.0))

(event `ChangeWeather_SandDustCalm`
  ;[1 1 1] ChangeWeather
  (`self.ChangeWeather` "/Game/UltraDynamicSky/Blueprints/Weather_Effects/Weather_Presets/Sand_Dust_Calm.Sand_Dust_Calm" 5.0))

(event `ChangeWeather_Cloudy`
  ;[1 1 1] ChangeWeather
  (`self.ChangeWeather` "/Game/UltraDynamicSky/Blueprints/Weather_Effects/Weather_Presets/Cloudy.Cloudy" 5.0))

(event `ChangeWeather_Rain`
  ;[1 1 1] ChangeWeather
  (`self.ChangeWeather` "/Game/UltraDynamicSky/Blueprints/Weather_Effects/Weather_Presets/Rain.Rain" 5.0))

(event `ChangeWeather_SandDustStorm`
  ;[1 1 1] ChangeWeather
  (`self.ChangeWeather` "/Game/UltraDynamicSky/Blueprints/Weather_Effects/Weather_Presets/Sand_Dust_Storm.Sand_Dust_Storm" 5.0))

(event `ChangeWeather_Foggy`
  ;[1 1 1] ChangeWeather
  (`self.ChangeWeather` "/Game/UltraDynamicSky/Blueprints/Weather_Effects/Weather_Presets/Foggy.Foggy" 5.0))

(event `ChangeWeather_RainLight`
  ;[1 1 1] ChangeWeather
  (`self.ChangeWeather` "/Game/UltraDynamicSky/Blueprints/Weather_Effects/Weather_Presets/Rain_Light.Rain_Light" 5.0))

(event `ChangeWeather_Snow`
  ;[1 1 1] ChangeWeather
  (`self.ChangeWeather` "/Game/UltraDynamicSky/Blueprints/Weather_Effects/Weather_Presets/Snow.Snow" 5.0))

(event `ChangeWeather_OverCast`
  ;[1 1 1] ChangeWeather
  (`self.ChangeWeather` "/Game/UltraDynamicSky/Blueprints/Weather_Effects/Weather_Presets/Overcast.Overcast" 5.0))

(event `ChangeWeather_RainThunderStorm`
  ;[1 1 1] ChangeWeather
  (`self.ChangeWeather` "/Game/UltraDynamicSky/Blueprints/Weather_Effects/Weather_Presets/Rain_Thunderstorm.Rain_Thunderstorm" 5.0))

(event `ChangeWeather_Blizzard`
  ;[1 1 1] ChangeWeather
  (`self.ChangeWeather` "/Game/UltraDynamicSky/Blueprints/Weather_Effects/Weather_Presets/Snow_Blizzard.Snow_Blizzard" 5.0))

(event `ChangeWeather_SnowLight`
  ;[1 1 1] ChangeWeather
  (`self.ChangeWeather` "/Game/UltraDynamicSky/Blueprints/Weather_Effects/Weather_Presets/Snow_Light.Snow_Light" 5.0))

(fn `GetWeatherAndCityInfo`
  (returns (City :type String) (weather :type String) (temperature :type String) (winddirection :type String) (windpower :type String))
  (bind _bp_component_varest (`self.BP_Component_VaRest`))
  (return (`/Game/BP/Component/BP_Component_VaRest.City` _bp_component_varest) (`/Game/BP/Component/BP_Component_VaRest.weather` _bp_component_varest) (`/Game/BP/Component/BP_Component_VaRest.temperature` _bp_component_varest) (`/Game/BP/Component/BP_Component_VaRest.winddirection` _bp_component_varest) (`/Game/BP/Component/BP_Component_VaRest.windpower` _bp_component_varest)))

(fn `UserConstructionScript`)